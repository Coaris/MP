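; BP_SamuraiController is the player controller that routes look and move input to the samurai character.
; On BeginPlay it caches the player character and adds the IMC_SamuraiGameplay mapping context to the Enhanced Input subsystem.
; The IA_Look and IA_Move actions forward their X and Y axis values to the character through message calls, leaving the movement and camera logic outside the controller.
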(event Input|EnhancedActionEvents|EnhancedInputActionIA_Look
  (params (ActionValue :type Vector%202D%20Structure) (ElapsedSeconds :type Float%20%28double-precision%29) (TriggeredSeconds :type Float%20%28double-precision%29) (InputAction :type Input%20Action%20Object%20Reference :default "/Game/Jiale/Input/IA_Look.IA_Look"))
  ;[1 1 1] Camera look
  (:Triggered
    (Class|BPISamurai|Look(Message) (Variables|Default|GetSamurai) (.x ActionValue) (.y ActionValue))))

(event Input|EnhancedActionEvents|EnhancedInputActionIA_Move
  (params (ActionValue :type Vector%202D%20Structure) (ElapsedSeconds :type Float%20%28double-precision%29) (TriggeredSeconds :type Float%20%28double-precision%29) (InputAction :type Input%20Action%20Object%20Reference :default "/Game/Jiale/Input/IA_Move.IA_Move"))
  ;[1 1 1] Move
  (:Triggered
    (Class|BPISamurai|Move(Message) (Variables|Default|GetSamurai) (.x ActionValue) (.y ActionValue))))

(event EventBeginPlay
  (bind _self self)
  (bind _returnvalue (PlayerController|LocalPlayerSubsystems|GetEnhancedInputLocalPlayerSubsystem _self))
  ;[1 1 1] Get player reference
  (Variables|Default|SetSamurai (Game|GetPlayerCharacter 0))
  ;[1 1 1] Add enhanced input system
  (Utilities|IsValid _returnvalue
    (:Is%20Valid
      (Input|AddMappingContext _returnvalue "/Game/Jiale/Input/IMC_SamuraiGameplay.IMC_SamuraiGameplay" 0 "(bIgnoreAllPressedKeysUntilRelease=True,bForceImmediately=False)"))))

(fn ConstructionScript)